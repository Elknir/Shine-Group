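; BP_FightManager links a combat encounter to its UI, covering fight start, health display and fight end.
; StartFight calls CombatStart with both base health values, sets a hardcoded slime enemy name and reads the player's name from GameInstance save data through BPI_SaveInterface.
; UpdateUI pushes health changes to the player and enemy widgets, and OnFightFinished forwards the win or loss result to the linked menu.
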(event `self.ReceiveBeginPlay`)

(event `self.OnFightFinished`
  (params (HasPlayerWon :type Boolean))
  (`/Game/Widgets/CAW_FightMenu.OnFightEnded` (`self.LinkedMenu`) HasPlayerWon))

(event `self.UpdateUI`
  (params (PlayerHealth :type Integer) (EnemyHealth :type Integer))
  ; Update HP after a hit
  (`/Game/Widgets/CAW_CharaStats.Set HP` (`self.UI Player`) PlayerHealth)
  (`/Game/Widgets/CAW_CharaStats.Set HP` (`self.UI Enemy`) EnemyHealth))

(event `Start Fight`
  (bind _returnvalue (`GameplayStatics.GetGameInstance`))
  ; Init Combat UI
  (`self.CombatStart` (`self.PlayerHeath`) (`self.EnemyHealth`))
  (`/Game/Widgets/CAW_CharaStats.Set Name` (`self.UI Enemy`) "Slime Très Méchant")
  ;; Get Save
  (if (`KismetSystemLibrary.DoesImplementInterface` _returnvalue "/Game/Save/BPI_SaveInterface.BPI_SaveInterface_C")
    (bind _save_game_data (message `/Game/Save/BPI_SaveInterface.Get Game Data` _returnvalue))
    (`/Game/Widgets/CAW_CharaStats.Set Name` (`self.UI Player`) (`/Game/Save/BP_ShineSaveGame.Character Name` _save_game_data))))

(fn `UserConstructionScript`)